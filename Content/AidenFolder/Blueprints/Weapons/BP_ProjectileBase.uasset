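; BP_ProjectileBase is a base weapon projectile that damages what it overlaps.
; Its construction script copies the Speed and GravityEffect variables into the ProjectileMovement component's initial speed, max speed and gravity scale.
; On overlap it ignores actors tagged Player or Bullet, applies Damage to any other actor, then destroys itself.
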(event EventBeginPlay
  (|CallParentFunction) ; This node is disabled and will not be called.\nDrag off pins to build functionality.
)

(event Collision|EventActorBeginOverlap
  (params (OtherActor :type Actor%20Object%20Reference))
  (|CallParentFunction OtherActor)
  (if (not (Actor|ActorHasTag OtherActor "Player"))
    (if (not (Actor|ActorHasTag OtherActor "Bullet"))
      (Game|Damage|ApplyDamage OtherActor (Variables|Default|GetDamage) 0 self)
      (Actor|DestroyActor))))

(event EventTick
  (params (DeltaSeconds :type Float%20%28single-precision%29))
  (|CallParentFunction DeltaSeconds) ; This node is disabled and will not be called.\nDrag off pins to build functionality.
)

(fn ConstructionScript
  (bind _projectilemovement (Variables|Default|GetProjectileMovement))
  (bind _speed (Variables|Default|GetSpeed))
  (|CallParentFunction)
  (Variables|/Script/Engine.ProjectileMovementComponent|SetMaxSpeed _projectilemovement _speed)
  (Variables|/Script/Engine.ProjectileMovementComponent|SetInitialSpeed _projectilemovement _speed)
  (Variables|/Script/Engine.ProjectileMovementComponent|SetProjectileGravityScale _projectilemovement (Variables|Default|GetGravityEffect)))