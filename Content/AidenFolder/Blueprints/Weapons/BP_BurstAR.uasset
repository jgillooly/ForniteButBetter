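; Burst assault rifle weapon Blueprint that overrides Fire to shoot one BP_BurstBullet projectile per call.
; Fire runs the parent logic, then spawns the bullet at the Arrow component's location.
; Bullet rotation follows the deprojected screen-center ray of player 0, with slight random spread, rather than converging from the muzzle onto an aim point.
; No burst timing or other event logic lives in this Blueprint.
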(event EventBeginPlay)

(event Collision|EventActorBeginOverlap
  (params (OtherActor :type Actor%20Object%20Reference)))

(event EventTick
  (params (DeltaSeconds :type Float%20%28single-precision%29)))

(fn ConstructionScript)

(fn Fire
  (bind _returnvalue (Viewport|GetViewportSize))
  (bind _returnvalue_2 (Game|GetPlayerController 0))
  (bind _returnvalue_3 (/ _returnvalue "(X=2.000000,Y=2.000000)"))
  (bind (_worldposition _worlddirection) (Class|GameplayStatics|DeprojectScreentoWorld _returnvalue_2 _returnvalue_3))
  (bind _returnvalue_4 (* _worlddirection 1e+03))
  (bind _returnvalue_5 (+ _returnvalue_4 _worldposition))
  (bind _returnvalue_6 (Math|Rotator|FindLookatRotation _worldposition _returnvalue_5))
  (|CallParentFunction)
  (Game|SpawnActorfromClass "/Game/AidenFolder/Blueprints/Weapons/BP_BurstBullet.BP_BurstBullet_C" (Math|Transform|MakeTransform (Transformation|GetWorldLocation (Variables|Default|GetArrow)) (Math|Rotator|MakeRotator (+ (.roll _returnvalue_6) (Math|Random|RandomFloatinRange -0.25 0.25)) (+ (.pitch _returnvalue_6) (Math|Random|RandomFloatinRange -0.25 0.25)) (+ (.yaw _returnvalue_6) (Math|Random|RandomFloatinRange -0.25 0.25))) "1.000000,1.000000,1.000000") "Undefined" "MultiplyWithRoot" 0 0))