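; Gold Scar weapon Blueprint that overrides its parent's Fire function to supply its own shot data.
; After the parent call, Fire returns the Arrow component's location, an aim rotation and BP_GoldScarBullet as the projectile class.
; The rotation follows a ray deprojected from the viewport center, with slight random spread on each axis, rather than the muzzle's facing.
; An unconnected BP_BurstBullet spawn node remains in Fire and never runs.
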(event EventBeginPlay
  (|CallParentFunction) ; This node is disabled and will not be called.\nDrag off pins to build functionality.
)

(event Collision|EventActorBeginOverlap
  (params (OtherActor :type Actor%20Object%20Reference))
  (|CallParentFunction OtherActor) ; This node is disabled and will not be called.\nDrag off pins to build functionality.
)

(event EventTick
  (params (DeltaSeconds :type Float%20%28single-precision%29))
  (|CallParentFunction DeltaSeconds) ; This node is disabled and will not be called.\nDrag off pins to build functionality.
)

(fn ConstructionScript
  (|CallParentFunction))

(fn Fire
  (bind _returnvalue (Viewport|GetViewportSize))
  (bind _returnvalue_2 (Game|GetPlayerController 0))
  (bind _returnvalue_3 (/ _returnvalue "(X=2.000000,Y=2.000000)"))
  (bind (_worldposition _worlddirection) (Class|GameplayStatics|DeprojectScreentoWorld _returnvalue_2 _returnvalue_3))
  (bind _returnvalue_4 (* _worlddirection 1e+03))
  (bind _returnvalue_5 (+ _returnvalue_4 _worldposition))
  (bind _returnvalue_6 (Math|Rotator|FindLookatRotation _worldposition _returnvalue_5))
  (|CallParentFunction)
  (return (Utilities|Array|MakeArray (Transformation|GetWorldLocation (Variables|Default|GetArrow))) (Utilities|Array|MakeArray (Math|Rotator|MakeRotator (+ (.roll _returnvalue_6) (Math|Random|RandomFloatinRange -0.05 0.05)) (+ (.pitch _returnvalue_6) (Math|Random|RandomFloatinRange -0.05 0.05)) (+ (.yaw _returnvalue_6) (Math|Random|RandomFloatinRange -0.05 0.05)))) "/Game/AidenFolder/Blueprints/Weapons/Ammo/BP_GoldScarBullet.BP_GoldScarBullet_C"))