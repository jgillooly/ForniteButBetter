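; Shotgun weapon Blueprint that overrides Fire to shoot a spread of projectiles after calling the parent's Fire.
; Each class entry in the NumBullets array spawns one actor at the Arrow component's location.
; Aim comes from deprojecting the screen center of player 0, with random roll, pitch and yaw offsets per spawn.
; The aim rotation is measured from the deprojected camera point, not from the Arrow.
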(event EventBeginPlay
  (|CallParentFunction) ; This node is disabled and will not be called.\nDrag off pins to build functionality.
)

(event Collision|EventActorBeginOverlap
  (params (OtherActor :type Actor%20Object%20Reference))
  (|CallParentFunction OtherActor) ; This node is disabled and will not be called.\nDrag off pins to build functionality.
)

(event EventTick
  (params (DeltaSeconds :type Float%20%28single-precision%29))
  (|CallParentFunction DeltaSeconds) ; This node is disabled and will not be called.\nDrag off pins to build functionality.
)

(fn ConstructionScript
  (|CallParentFunction))

(fn Fire
  (bind _returnvalue (Viewport|GetViewportSize))
  (bind _returnvalue_2 (Game|GetPlayerController 0))
  (bind _returnvalue_3 (/ _returnvalue "(X=2.000000,Y=2.000000)"))
  (bind (_worldposition _worlddirection) (Class|GameplayStatics|DeprojectScreentoWorld _returnvalue_2 _returnvalue_3))
  (bind _returnvalue_4 (* _worlddirection 1e+03))
  (bind _returnvalue_5 (+ _returnvalue_4 _worldposition))
  (bind _returnvalue_6 (Math|Rotator|FindLookatRotation _worldposition _returnvalue_5))
  (|CallParentFunction)
  (for _array_element (Variables|Default|GetNumBullets)
    (Game|SpawnActorfromClass _array_element (Math|Transform|MakeTransform (Transformation|GetWorldLocation (Variables|Default|GetArrow)) (Math|Rotator|MakeRotator (+ (.roll _returnvalue_6) (Math|Random|RandomFloatinRange -1e+01 1e+01)) (+ (.pitch _returnvalue_6) (Math|Random|RandomFloatinRange -1e+01 1e+01)) (+ (.yaw _returnvalue_6) (Math|Random|RandomFloatinRange -1e+01 1e+01))) "1.000000,1.000000,1.000000") "Undefined" "MultiplyWithRoot" 0 0)))