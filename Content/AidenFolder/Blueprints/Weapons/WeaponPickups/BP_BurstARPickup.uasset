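; Burst AR weapon pickup that swaps itself for another pickup actor when its PickupType is set to a different handled weapon.
; Every Tick, an if chain tests PickupType for pistol, SMG, shotgun or sniper, spawns a replacement at its own transform, then destroys itself.
; Only the pistol and SMG branches set a class to spawn; the shotgun and sniper spawns have none.
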(event EventBeginPlay)

(event Collision|EventActorBeginOverlap
  (params (OtherActor :type Actor%20Object%20Reference)))

(event Collision|EventActorEndOverlap
  (params (OtherActor :type Actor%20Object%20Reference)))

(event EventTick
  (params (DeltaSeconds :type Float%20%28single-precision%29))
  (bind _returnvalue (Transformation|GetActorTransform))
  (bind _pickuptype (Variables|Default|GetPickupType))
  (if (== _pickuptype "/Game/AidenFolder/Blueprints/Weapons/BP_Pistol.BP_Pistol_C")
    (Game|SpawnActorfromClass "/Game/AidenFolder/Blueprints/Weapons/WeaponPickups/BP_PistolPickup.BP_PistolPickup_C" _returnvalue "Undefined" "MultiplyWithRoot" 0 0)
    (Actor|DestroyActor)
    (elif (== _pickuptype "/Game/AidenFolder/Blueprints/Weapons/BP_SMG.BP_SMG_C")
      (Game|SpawnActorfromClass "/Game/AidenFolder/Blueprints/Weapons/WeaponPickups/BP_SMGPickup.BP_SMGPickup_C" _returnvalue "Undefined" "MultiplyWithRoot" 0 0)
      (Actor|DestroyActor)
      (elif (== _pickuptype "/Game/AidenFolder/Blueprints/Weapons/BP_Shotgun.BP_Shotgun_C")
        (Game|SpawnActorfromClass "/Game/AidenFolder/Blueprints/Weapons/WeaponPickups/BP_ShotgunPickup.BP_ShotgunPickup_C" _returnvalue "Undefined" "MultiplyWithRoot" 0 0)
        (Actor|DestroyActor)
        (elif (== _pickuptype "/Game/AidenFolder/Blueprints/Weapons/BP_Sniper.BP_Sniper_C")
          (Game|SpawnActorfromClass "/Game/AidenFolder/Blueprints/Weapons/WeaponPickups/BP_SniperPickup.BP_SniperPickup_C" _returnvalue "Undefined" "MultiplyWithRoot" 0 0)
          (Actor|DestroyActor))))))

(fn ConstructionScript)