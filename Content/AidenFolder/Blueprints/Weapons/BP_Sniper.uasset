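; BP_Sniper is a sniper weapon Blueprint that overrides its parent's Fire function to supply the shot's origin, direction and projectile class.
; Fire calls the parent, then returns the Arrow component's location, an aim rotation and the BP_SniperBullet class.
; The rotation follows the ray deprojected from player 0's screen center, so it matches the view direction rather than converging from the Arrow.
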(event EventBeginPlay)

(event Collision|EventActorBeginOverlap
  (params (OtherActor :type Actor%20Object%20Reference)))

(event EventTick
  (params (DeltaSeconds :type Float%20%28single-precision%29)))

(fn ConstructionScript)

(fn Fire
  (bind _returnvalue (Viewport|GetViewportSize))
  (bind _returnvalue_2 (Game|GetPlayerController 0))
  (bind _returnvalue_3 (/ _returnvalue "(X=2.000000,Y=2.000000)"))
  (bind (_worldposition _worlddirection) (Class|GameplayStatics|DeprojectScreentoWorld _returnvalue_2 _returnvalue_3))
  (|CallParentFunction)
  (return (Utilities|Array|MakeArray (Transformation|GetWorldLocation (Variables|Default|GetArrow))) (Utilities|Array|MakeArray (Math|Rotator|FindLookatRotation _worldposition (+ (* _worlddirection 1e+03) _worldposition))) "/Game/AidenFolder/Blueprints/Weapons/Ammo/BP_SniperBullet.BP_SniperBullet_C"))